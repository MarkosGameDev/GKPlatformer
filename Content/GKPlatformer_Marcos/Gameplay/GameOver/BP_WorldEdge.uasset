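; BP_WorldEdge is a level boundary actor that triggers defeat when the player's combat mech hits its Box collider.
; The hit handler casts to BP_CombatMech_M and starts the AM_Death montage on its mesh.
; It then removes the mech's input mapping context, adds the WBP_Defeat_M widget to the viewport and shows the mouse cursor, while setting input mode to game only.
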(event OnComponentHit(Box)
  (params (HitComponent :type Primitive%20Component%20Object%20Reference) (OtherActor :type Actor%20Object%20Reference) (OtherComp :type Primitive%20Component%20Object%20Reference) (NormalImpulse :type Vector :default "0, 0, 0") (Hit :type Hit%20Result%20Structure%20%28by%20ref%29))
  (bind _asbp_combat_mech_m (Utilities|Casting|CastToBP_CombatMech_M OtherActor))
  (Animation|Montage|PlayMontage (Variables|/Script/Engine.Character|GetMesh _asbp_combat_mech_m) "/Game/GKPlatformer/Gameplay/Character/Animations/AM_Death.AM_Death"
    (:then
      (Input|RemoveMappingContext (PlayerController|LocalPlayerSubsystems|GetEnhancedInputLocalPlayerSubsystem (Game|GetPlayerController 0)) "/Game/GKPlatformer_Marcos/Gameplay/Input/IMC_CombatMech_M.IMC_CombatMech_M" "(bIgnoreAllPressedKeysUntilRelease=True,bForceImmediately=False,bNotifyUserSettings=False)")
      (bind _returnvalue (UserInterface|CreateWidget "/Game/GKPlatformer_Marcos/Gameplay/UI/WBP_Defeat_M.WBP_Defeat_M_C" (Game|GetPlayerController 0)))
      (UserInterface|Viewport|AddtoViewport _returnvalue 0)
      (Variables|/Script/Engine.PlayerController|SetbShowMouseCursor (Game|GetPlayerController 0) true)
      (Input|SetInputModeGameOnly (Game|GetPlayerController 0) false))))

(event EventBeginPlay)

(event Collision|EventActorBeginOverlap
  (params (OtherActor :type Actor%20Object%20Reference)))

(event EventTick
  (params (DeltaSeconds :type Float%20%28single-precision%29)))

(fn ConstructionScript)