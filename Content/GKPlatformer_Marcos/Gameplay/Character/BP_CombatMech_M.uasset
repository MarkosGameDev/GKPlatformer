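; BP_CombatMech_M is a playable mech character for a platformer, handling movement and jumping through Enhanced Input.
; BeginPlay adds its input mapping context to the first player's controller, and the movement action drives strafe and forward input relative to control rotation, ignoring pitch.
; The jump action triggers a jump and restarts a timeline that animates CharacterMovement gravity scale to shape the jump arc.
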(event Input|EnhancedActionEvents|EnhancedInputActionIA_Movement_M
  (params (ActionValue :type Vector%202D%20Structure) (ElapsedSeconds :type Float%20%28double-precision%29) (TriggeredSeconds :type Float%20%28double-precision%29) (InputAction :type Input%20Action%20Object%20Reference :default "/Game/GKPlatformer_Marcos/Gameplay/Input/Actions/IA_Movement_M.IA_Movement_M"))
  (bind _returnvalue (Pawn|GetControlRotation :!class /Script/Engine.Pawn))
  (Pawn|Input|AddMovementInput (Math|Vector|GetRightVector (Math|Rotator|MakeRotator (.roll _returnvalue) 0.0 (.yaw _returnvalue))) (.x ActionValue) false)
  (Pawn|Input|AddMovementInput (Math|Vector|GetForwardVector (Math|Rotator|MakeRotator 0.0 0.0 (.yaw (Pawn|GetControlRotation :!class /Script/Engine.Pawn)))) (.y ActionValue) false))

(event Input|EnhancedActionEvents|EnhancedInputActionIA_Jump_M
  (params (ActionValue :type Boolean) (ElapsedSeconds :type Float%20%28double-precision%29) (TriggeredSeconds :type Float%20%28double-precision%29) (InputAction :type Input%20Action%20Object%20Reference :default "/Game/GKPlatformer_Marcos/Gameplay/Input/Actions/IA_Jump_M.IA_Jump_M"))
  (Character|Jump)
  (bind _gravity (Timeline|JumpTimeline PlayFromStart)
    (:Update
      (Variables|/Script/Engine.CharacterMovementComponent|SetGravityScale (Variables|Character|GetCharacterMovement) _gravity))))

(event EventBeginPlay
  (Input|AddMappingContext (PlayerController|LocalPlayerSubsystems|GetEnhancedInputLocalPlayerSubsystem (Game|GetPlayerController 0)) "/Game/GKPlatformer_Marcos/Gameplay/Input/IMC_CombatMech_M.IMC_CombatMech_M" 0 "(bIgnoreAllPressedKeysUntilRelease=True,bForceImmediately=False,bNotifyUserSettings=False)"))

(fn ConstructionScript)