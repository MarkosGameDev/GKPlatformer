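; Coin placer actor that lays a row of BP_Coin_M coins along its spline.
; Generate destroys existing child actors, then spawns coins spaced by spline length over QtdeCoin, using local-space positions.
; Each coin gets a faster Idle sequence play rate and is attached to the actor with relative rules.
; Clear destroys every BP_Coin_M in the world, not just this spline's coins.
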(event Custom|Generate
  (Utilities|FlowControl|Sequence
    (:then_0
      (for _array_element (Actor|GetAllChildActors true)
        (Actor|DestroyActor _array_element)))
    (:then_1
      (for _index (range 0 (Variables|Default|GetQtdeCoin))
        (bind _returnvalue (Game|SpawnActorfromClass "/Game/GKPlatformer_Marcos/Gameplay/Coin/GoldenCoin/BP_Coin_M.BP_Coin_M_C" (Math|Transform|MakeTransform (Spline|GetLocationatDistanceAlongSpline (Variables|Default|GetSpline) (Math|Conversions|ToFloat(Integer) (* _index (/ (Spline|GetSplineLength (Variables|Default|GetSpline)) (Variables|Default|GetQtdeCoin)))) "Local") "0, 0, 0" "1.000000,1.000000,1.000000") "Undefined" "MultiplyWithRoot" 0 0))
        (Components|Timeline|SetPlayRate (Variables|/Script/ActorSequence.ActorSequenceComponent|GetSequencePlayer (Variables|/Game/GKPlatformer_Marcos/Gameplay/Coin/GoldenCoin/BP_Coin_M.BP_Coin_M_C|GetIdle _returnvalue)) 5.0)
        (Transformation|AttachActorToActor _returnvalue self "None" "KeepRelative" "KeepRelative" "KeepRelative" true)))))

(event Custom|Clear
  (bind _outactors (Actor|GetAllActorsOfClass "/Game/GKPlatformer_Marcos/Gameplay/Coin/GoldenCoin/BP_Coin_M.BP_Coin_M_C"))
  (for _array_element _outactors
    (Actor|DestroyActor _array_element)))

(event EventBeginPlay)

(event Collision|EventActorBeginOverlap
  (params (OtherActor :type Actor%20Object%20Reference)))

(event EventTick
  (params (DeltaSeconds :type Float%20%28single-precision%29)))

(fn ConstructionScript)