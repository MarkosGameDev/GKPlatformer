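; BP_Flag is a goal flag that triggers the win sequence when a BP_CombatMech_M overlaps its Sphere.
; It starts a cheering montage on the mech and, without waiting for it to finish, removes the mech's Enhanced Input mapping context.
; It then creates a container widget, pushes the winner prompt onto it and shows the mouse cursor, while setting input mode to game only.
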(event OnComponentBeginOverlap(Sphere)
  (params (OverlappedComponent :type Primitive%20Component%20Object%20Reference) (OtherActor :type Actor%20Object%20Reference) (OtherComp :type Primitive%20Component%20Object%20Reference) (OtherBodyIndex :type Integer) (bFromSweep :type Boolean) (SweepResult :type Hit%20Result%20Structure%20%28by%20ref%29))
  (bind _asbp_combat_mech_m (Utilities|Casting|CastToBP_CombatMech_M OtherActor))
  (Animation|Montage|PlayMontage (Variables|/Script/Engine.Character|GetMesh _asbp_combat_mech_m) "/Game/GKPlatformer/Gameplay/Character/Animations/AM_Cheering.AM_Cheering"
    (:then
      (Input|RemoveMappingContext (PlayerController|LocalPlayerSubsystems|GetEnhancedInputLocalPlayerSubsystem (Game|GetPlayerController 0)) "/Game/GKPlatformer_Marcos/Gameplay/Input/IMC_CombatMech_M.IMC_CombatMech_M" "(bIgnoreAllPressedKeysUntilRelease=True,bForceImmediately=False,bNotifyUserSettings=False)")
      (bind _returnvalue (UserInterface|CreateWidget "/Game/GKPlatformer_Marcos/MainMenu/UI/WBP_Container.WBP_Container_C" (Game|GetPlayerController 0)))
      (bind _output_get (Variables|Default|SetPromptBase _returnvalue))
      (UserInterface|Viewport|AddtoViewport _output_get 0)
      (Default|PushPrompt (Variables|Default|GetPromptBase) "/Game/GKPlatformer_Marcos/Gameplay/UI/WBP_Winner_M2.WBP_Winner_M2_C")
      (Variables|/Script/Engine.PlayerController|SetbShowMouseCursor (Game|GetPlayerController 0) true)
      (Input|SetInputModeGameOnly (Game|GetPlayerController 0) false))))

(event EventBeginPlay)

(event Collision|EventActorBeginOverlap
  (params (OtherActor :type Actor%20Object%20Reference)))

(event EventTick
  (params (DeltaSeconds :type Float%20%28single-precision%29)))

(fn ConstructionScript)