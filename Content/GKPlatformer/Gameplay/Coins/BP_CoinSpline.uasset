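; BP_CoinSpline is a coin placer that lays out a row of BP_Coin actors along a spline.
; Its Generate event destroys all child actors, then spawns QtdMoedas coins at equal distance steps, ending at the spline's end with none at its start.
; Coins spawn at spline-local coordinates and attach with KeepRelative, so those coordinates become offsets from the placer.
; The construction script is empty, so placement happens only when Generate runs.
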(event Custom|Generate
  (Utilities|FlowControl|Sequence
    (:then_0
      (for _array_element (Actor|GetAllChildActors true)
        (Actor|DestroyActor _array_element)))
    (:then_1
      (for _index (range 1 (Variables|Default|GetQtdMoedas))
        (bind _returnvalue (Game|SpawnActorfromClass "/Game/GKPlatformer/Gameplay/Coins/BP_Coin.BP_Coin_C" (Math|Transform|MakeTransform (Spline|GetLocationatDistanceAlongSpline (Variables|Default|GetSpline) (* (/ (Spline|GetSplineLength (Variables|Default|GetSpline)) (Variables|Default|GetQtdMoedas)) _index) "Local") "0, 0, 0" "1.000000,1.000000,1.000000") "Undefined" "MultiplyWithRoot" 0 0))
        (Transformation|AttachActorToActor _returnvalue self "None" "KeepRelative" "KeepRelative" "KeepRelative" true)))))

(fn ConstructionScript)